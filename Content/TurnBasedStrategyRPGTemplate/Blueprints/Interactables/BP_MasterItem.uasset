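; Base interactable pickup for the exploration hero in a turn-based RPG, acting by item type.
; An InteractionDetector child actor triggers a pausing info dialogue, then refills mana, expands inventory slots (bag) or stores the item or potion.
; Successful bag, item and potion pickups destroy the actor; Health has no pickup effect.
; Cursor hover swaps materials with sound, hero proximity plays audio, and Interact spawns a far-off Studio for inspection.
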(event `self.ReceiveBeginPlay`
  ;[1 1 1] Assign interaction events
  (`|ExecutionSequence`
    (:`then_0`
      (bind _asbp_interaction_detector (cast `/Game/TurnBasedStrategyRPGTemplate/Blueprints/Interactables/BP_InteractionDetector` (`ChildActorComponent.ChildActor` (`self.InteractionActor`))))
      (bind _output_get (set `self.interactionDetector` _asbp_interaction_detector))
      (add `/Game/TurnBasedStrategyRPGTemplate/Blueprints/Interactables/BP_InteractionDetector.OnInteracted` _output_get (delegate `OnInteractedHandler`))
      (add `/Game/TurnBasedStrategyRPGTemplate/Blueprints/Interactables/BP_InteractionDetector.OnLoaded` (`self.interactionDetector`) (delegate `OnLoadedHandler`)))
    (:`then_1`
      (bind _asbp_explore_hero (cast `/Game/TurnBasedStrategyRPGTemplate/Blueprints/Heroes/Explore/BP_ExploreHero` (`GameplayStatics.GetPlayerCharacter` 0)))
      (bind _output_get_2 (set `self.As BP Explore Hero` _asbp_explore_hero))
      (set `self.Inventory Component` (`/Game/TurnBasedStrategyRPGTemplate/Blueprints/Heroes/Explore/BP_ExploreHeroBase.InventoryComponent` _output_get_2)))
    (:`then_2`
      (setmembers `/Game/TurnBasedStrategyRPGTemplate/Blueprints/Interactables/Inventory/ItemStructure` :`StructRef` (`self.ItemStructure`) :`Mesh` (`StaticMeshComponent.StaticMesh` (`self.Item`)) :`Mesh1` (`StaticMeshComponent.StaticMesh` (`self.Item1`)) :`Mesh3` null :`Mesh4` null :`Mesh2` null))))

(event `OnInteractedHandler`
  (params (buttonIndex :type Integer))
  ;[1 1 1] Assign interaction events
  (`self.Interaction`))

(event `OnLoadedHandler`
  (params (shouldLoadEnemyPawns :type Boolean))
  ;[1 1 1] Assign interaction events
  (`self.OnShrineLoaded`))

(event `Interaction`
  (bind _as_bp_explore_hero (`self.As BP Explore Hero`))
  (bind ((`ItemName_2_4E5B1D31467E1D538578D7B20F1C751A` _itemname) (`BenefitDescription_64_B4377F5943F29926018D8E8897D5097F` _benefitdescription)) (break `/Game/TurnBasedStrategyRPGTemplate/Blueprints/Interactables/Inventory/ItemStructure` (`self.ItemStructure`)))
  ;[0.3196 0.1789 1 1 60] Interaction
  (bind _returnvalue (`|CreateWidget` "/Game/TurnBasedStrategyRPGTemplate/Blueprints/Widgets/ExploreWidgets/WBP_InfoDialogue.WBP_InfoDialogue_C" null _itemname _benefitdescription "Ok"))
  (`UserWidget.AddToViewport` _returnvalue 0)
  (add `/Game/TurnBasedStrategyRPGTemplate/Blueprints/Widgets/ExploreWidgets/WBP_InfoDialogue.OnOkClicked` _returnvalue (delegate `OnDialogueClosed`))
  (`GameplayStatics.SetGamePaused` true)
  (switch `/Game/TurnBasedStrategyRPGTemplate/Blueprints/Interactables/E_ItemType` (`self.ItemType`)
    (:`NewEnumerator0`
      (`/Game/TurnBasedStrategyRPGTemplate/Blueprints/Heroes/Explore/BP_ExploreHeroBase.SetFullMana` _as_bp_explore_hero))
    (:`NewEnumerator2`
      (bind _success (`self.PickUpBenefits`))
      (if _success
        (`KismetSystemLibrary.RetriggerableDelay` 0.2)
        (`self.K2_DestroyActor`)))
    (:`NewEnumerator4`
      (bind _success_2 (`/Game/TurnBasedStrategyRPGTemplate/Blueprints/Interactables/Inventory/InventoryComponent.AddToInventory` (`/Game/TurnBasedStrategyRPGTemplate/Blueprints/Heroes/Explore/BP_ExploreHeroBase.InventoryComponent` _as_bp_explore_hero) (make `/Game/TurnBasedStrategyRPGTemplate/Blueprints/Interactables/Inventory/SlotStructure` (`self.ItemStructure`) 1) :!label _label))
      (if _success_2
        (`KismetSystemLibrary.RetriggerableDelay` 0.2)
        (`self.K2_DestroyActor`)))
    (:`NewEnumerator5`
      (goto _label))))

(event `OnDialogueClosed`
  ;[0.3196 0.1789 1 1 60] Interaction
  (`Widget.RemoveFromParent` (stale `Interaction` _returnvalue))
  (`/Game/TurnBasedStrategyRPGTemplate/Blueprints/Interactables/BP_InteractionDetector.EnableInteraction` (`self.interactionDetector`))
  (`GameplayStatics.SetGamePaused` false))

(event `OnShrineLoaded`
  ;[1 1 1] Enable interaction after load
  (`/Game/TurnBasedStrategyRPGTemplate/Blueprints/Interactables/BP_InteractionDetector.EnableInteraction` (`self.interactionDetector`)))

(event `/Game/TopDownBP/Blueprints/Interface/InspectInterface.Interact`
  (params (Player :type "/Game/TurnBasedStrategyRPGTemplate/Blueprints/Heroes/Explore/BP_ExploreHeroBase Object Reference"))
  (bind (_itemname _itemdescription) (break `/Game/TurnBasedStrategyRPGTemplate/Blueprints/Interactables/Inventory/ItemStructure` (`self.ItemStructure`)))
  (bind _returnvalue (`|SpawnActorFromClass` "/Game/TurnBasedStrategyRPGTemplate/Blueprints/Interactables/Inventory/Studio.Studio_C" (`KismetMathLibrary.MakeTransform` (1000000000.0 0.0 0.0)) "Undefined" "OverrideRootScale" null (struct) null))
  (message `/Game/TopDownBP/Blueprints/Interface/InspectInterface.Inspect` _returnvalue Player _itemname _itemdescription (`StaticMeshComponent.StaticMesh` (`self.Item`)) (`StaticMeshComponent.StaticMesh` (`self.Item1`)) null null null false null (struct)))

(event `self.Sphere.OnComponentBeginOverlap`
  (params (OverlappedComponent :type "PrimitiveComponent Object Reference") (OtherActor :type "Actor Object Reference") (OtherComp :type "PrimitiveComponent Object Reference") (OtherBodyIndex :type Integer) (bFromSweep :type Boolean) (SweepResult :type "HitResult Structure (by ref)"))
  (cast `/Game/TurnBasedStrategyRPGTemplate/Blueprints/Heroes/Explore/BP_ExploreHero` OtherActor)
  (bind _returnvalue (`GameplayStatics.SpawnSoundAtLocation` (`|GetArrayItem` (`self.ItemSoundsArray`) (`self.SoundIndex`)) (`self.K2_GetActorLocation`) (struct) 1.0 1.0 0.0 null null))
  (set `self.SpawnedSound` _returnvalue))

(event `self.Sphere.OnComponentEndOverlap`
  (params (OverlappedComponent :type "PrimitiveComponent Object Reference") (OtherActor :type "Actor Object Reference") (OtherComp :type "PrimitiveComponent Object Reference") (OtherBodyIndex :type Integer))
  (cast `/Game/TurnBasedStrategyRPGTemplate/Blueprints/Heroes/Explore/BP_ExploreHero` OtherActor)
  (bind _spawnedsound (`self.SpawnedSound`)
    (:`then`
      (`AudioComponent.Stop` _spawnedsound))
    (:`else`)))

(event `self.Item.OnBeginCursorOver`
  (params (TouchedComponent :type "PrimitiveComponent Object Reference"))
  (bind _returnvalue (`self.K2_GetActorLocation`))
  (bind _item (`self.Item`))
  (switch `/Game/TurnBasedStrategyRPGTemplate/Blueprints/Interactables/E_ItemType` (`self.ItemType`)
    (:`NewEnumerator0`
      (`PrimitiveComponent.SetMaterial` _item 0 "/Engine/VREditor/UI/DiscMaterial.DiscMaterial")
      (`GameplayStatics.PlaySoundAtLocation` "/Game/TurnBasedStrategyRPGTemplate/Sounds/WAV_ButtonClick.WAV_ButtonClick" _returnvalue (struct) 1.0 1.0 0.0 null null null))
    (:`NewEnumerator1`
      (`PrimitiveComponent.SetMaterial` _item 0 "/Engine/VREditor/UI/FrameMaterial.FrameMaterial" :!label _label_2)
      (`PrimitiveComponent.SetMaterial` (`self.Item1`) 0 "/Engine/VREditor/UI/FrameMaterial.FrameMaterial")
      (`GameplayStatics.PlaySoundAtLocation` "/Game/TurnBasedStrategyRPGTemplate/Sounds/WAV_ButtonClick.WAV_ButtonClick" _returnvalue (struct) 1.0 1.0 0.0 null null null))
    (:`NewEnumerator2`
      (`PrimitiveComponent.SetMaterial` _item 0 "/Engine/EngineMaterials/EditorBrushMaterial.EditorBrushMaterial")
      (`GameplayStatics.PlaySoundAtLocation` "/Game/TopDownBP/Blueprints/Assets/Sounds/shumnyiy-sbros-ryukzaka-s-plecha.shumnyiy-sbros-ryukzaka-s-plecha" _returnvalue (struct) 1.0 1.0 0.0 null null null))
    (:`NewEnumerator4`
      (goto _label_2))
    (:`NewEnumerator5`
      (`PrimitiveComponent.SetMaterial` _item 0 "/Engine/VREditor/UI/FrameMaterial.FrameMaterial")
      (`PrimitiveComponent.SetMaterial` (`self.Item1`) 0 "/Engine/VREditor/UI/FrameMaterial.FrameMaterial")
      (`GameplayStatics.PlaySoundAtLocation` "/Game/TopDownBP/Blueprints/Assets/Sounds/zvon-steklyannyih-bokalov.zvon-steklyannyih-bokalov" _returnvalue (struct) 0.5 1.0 0.0 null null null))))

(event `self.Item.OnEndCursorOver`
  (params (TouchedComponent :type "PrimitiveComponent Object Reference"))
  (`PrimitiveComponent.SetMaterial` (`self.Item`) 0 null)
  (`PrimitiveComponent.SetMaterial` (`self.Item1`) 0 null))

(fn `CheckInspect`
  (returns (Success :type Boolean))
  (bind (_itemstructure_itemname _itemstructure_itemdescription _itemstructure_benefitdescription _itemstructure_socket _itemstructure_canbeadded) (break `/Game/TurnBasedStrategyRPGTemplate/Blueprints/Interactables/Inventory/ItemStructure` (`self.ItemStructure`)))
  (if _itemstructure_canbeadded
    (bind _asbp_explore_hero_base (cast `/Game/TurnBasedStrategyRPGTemplate/Blueprints/Heroes/Explore/BP_ExploreHeroBase` (`GameplayStatics.GetPlayerCharacter` 0)))
    (if (== 0 -1)
      _)
    (else
      (return true))))

(fn `PickUpBenefits`
  (returns (Success :type Boolean))
  (bind _asbp_explore_hero_base (cast `/Game/TurnBasedStrategyRPGTemplate/Blueprints/Heroes/Explore/BP_ExploreHeroBase` (`GameplayStatics.GetPlayerCharacter` 0)))
  (bind _inventorycomponent (`/Game/TurnBasedStrategyRPGTemplate/Blueprints/Heroes/Explore/BP_ExploreHeroBase.InventoryComponent` _asbp_explore_hero_base))
  (bind _output_get (set `/Game/TurnBasedStrategyRPGTemplate/Blueprints/Interactables/Inventory/InventoryComponent.NumberofSlots` (+ (`/Game/TurnBasedStrategyRPGTemplate/Blueprints/Interactables/Inventory/InventoryComponent.NumberofSlots` _inventorycomponent) 2) _inventorycomponent))
  (`KismetArrayLibrary.Array_Resize` (`/Game/TurnBasedStrategyRPGTemplate/Blueprints/Interactables/Inventory/InventoryComponent.SlotStructure(inventoryArray)` _inventorycomponent) _output_get)
  (`/Game/TurnBasedStrategyRPGTemplate/Blueprints/Interactables/Inventory/InventoryComponent.ToggleInventory` (`/Game/TurnBasedStrategyRPGTemplate/Blueprints/Heroes/Explore/BP_ExploreHeroBase.InventoryComponent` (`self.As BP Explore Hero`)))
  (`GameplayStatics.PlaySoundAtLocation` "/Game/TurnBasedStrategyRPGTemplate/Blueprints/Interactables/Inventory/Assets/zakrtie-starogo-ryibatskogo-ryukzaka.zakrtie-starogo-ryibatskogo-ryukzaka" (`self.K2_GetActorLocation` (`self.As BP Explore Hero`)) (struct) 1.0 1.0 0.0 null null null)
  (return true))

(fn `UseItem`
  (returns (Success :type Boolean))
  (`KismetSystemLibrary.PrintString` "Item Use")
  (return true))

(fn `UserConstructionScript`
  (`parent.UserConstructionScript`))